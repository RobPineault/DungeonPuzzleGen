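; Spike trap actor for the dungeon puzzle generator, with configurable left and right sides and optional movement.
; On BeginPlay, the Type enum and an inverting Flip flag decide, per side, whether walls and borders show or are replaced by open borders, plus supports on the right.
; When MovingSpikes is set, its ActorSequence plays after an Offset delay, allowing staggered timing.
; Logic to attach spheres to spear tips exists but is never executed.
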(event `self.ReceiveBeginPlay`
  (bind _flip (`self.flip`))
  (bind _type (`self.Type`))
  (bind _returnvalue (`|EnumEquality` _type "NewEnumerator1"))
  (`self.Hide Right` (xor (or _returnvalue (`|EnumEquality` _type "NewEnumerator2")) _flip))
  (`self.Hide Left` (xor (or (`|EnumEquality` _type "NewEnumerator0") _returnvalue) _flip))
  (if (`self.Moving Spikes`)
    (`KismetSystemLibrary.Delay` (`self.Offset`))
    (`MovieSceneSequencePlayer.Play` (`ActorSequenceComponent.SequencePlayer` (`self.ActorSequence`)))))

(fn `Hide Left`
  (params (Hide :type Boolean))
  (`SceneComponent.SetVisibility` (`self.Border TL`) (not Hide) false)
  (`SceneComponent.SetVisibility` (`self.Border BL`) (not Hide) false)
  (`SceneComponent.SetVisibility` (`self.Wall L`) (not Hide) false)
  (`SceneComponent.SetVisibility` (`self.Border TL Open`) Hide false)
  (`SceneComponent.SetVisibility` (`self.Border BL Open`) Hide false))

(fn `Hide Right`
  (params (Hide :type Boolean))
  (`SceneComponent.SetVisibility` (`self.Border TR`) (not Hide) false)
  (`SceneComponent.SetVisibility` (`self.Border BR`) (not Hide) false)
  (`SceneComponent.SetVisibility` (`self.Wall R`) (not Hide) false)
  (`SceneComponent.SetVisibility` (`self.Border TR Open`) Hide false)
  (`SceneComponent.SetVisibility` (`self.Border BR Open`) Hide false)
  (`SceneComponent.SetVisibility` (`self.Support1`) Hide false)
  (`SceneComponent.SetVisibility` (`self.Support`) Hide false))

(fn `UserConstructionScript`)