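; Tile actor for the dungeon puzzle generator that stores its grid coordinates and a reference to its spawning Blueprint.
; When set as the spawn tile, it spawns a first-person character above itself and has player 0 possess it.
; Helper functions build the tile at runtime by attaching static mesh components or spawned actors to named sockets, and find child components by socket name.
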(event `Set SpawnBP`
  (params (NewParam :type "/Game/DungeonPuzzleGen/Blueprints/SpawnBP Object Reference") (X :type Integer) (Y :type Integer))
  (set `self.X Coord` X)
  (set `self.Y Coord` Y)
  (set `self.SpawnBPRef` NewParam))

(event `Set As Spawn`
  (bind _returnvalue (`|SpawnActorFromClass` "/Game/FirstPerson/Blueprints/BP_FirstPersonCharacter.BP_FirstPersonCharacter_C" (`KismetMathLibrary.MakeTransform` (+ (.location (`self.GetTransform`)) (0.0 0.0 250.0)) (.rotation (`self.GetTransform`)) (.scale (`self.GetTransform`))) "Undefined" "OverrideRootScale" null null))
  (`Controller.Possess` (`GameplayStatics.GetPlayerController` 0) _returnvalue))

(fn `Create SMC From Comp`
  (params (`Comp Data` :type "/Game/DungeonPuzzleGen/Blueprints/TileComponentData Structure") (Parent :type "StaticMeshComponent Object Reference"))
  (returns (Child :type "StaticMeshComponent Object Reference"))
  (bind (_mesh _foliage _weight _socketname) (break `/Game/DungeonPuzzleGen/Blueprints/TileComponentData` `Comp Data`))
  (bind _returnvalue (`AddComponent|NODE_AddStaticMeshComponent-1` :`bManualAttachment` true))
  (`SceneComponent.K2_AttachToComponent` _returnvalue Parent _socketname "KeepRelative" "KeepRelative" "KeepRelative" true)
  (`StaticMeshComponent.SetStaticMesh` _returnvalue _mesh)
  (return _returnvalue))

(fn `Create SMC From Mesh`
  (params (Mesh :type "StaticMesh Object Reference") (Parent :type "StaticMeshComponent Object Reference") (Socket :type Name))
  (returns (Child :type "StaticMeshComponent Object Reference"))
  (bind _returnvalue (`AddComponent|NODE_AddStaticMeshComponent-0` :`bManualAttachment` true))
  (`SceneComponent.K2_AttachToComponent` _returnvalue Parent Socket "KeepRelative" "KeepRelative" "KeepRelative" true)
  (`StaticMeshComponent.SetStaticMesh` _returnvalue Mesh)
  (return _returnvalue))

(fn `Find Child by Socket`
  (params (Parent :type "StaticMeshComponent Object Reference") (Name :type Name))
  (returns (NewParam :type "SceneComponent Object Reference"))
  (for _array_element (`SceneComponent.GetChildrenComponents` Parent false)
    (if (== Name (`SceneComponent.GetAttachSocketName` _array_element))
      (return _array_element))))

(fn `Spawn Actor from SMC`
  (params (Class :type "Actor Class Reference") (Socket :type Name) (SMC :type "StaticMeshComponent Object Reference"))
  (returns (NewParam :type "Actor Object Reference"))
  (bind _returnvalue (`|SpawnActorFromClass` Class (`KismetMathLibrary.MakeTransform` (0.0 0.0 0.0)) "Undefined" "OverrideRootScale" null null))
  (`self.K2_AttachToComponent` _returnvalue SMC Socket "KeepRelative" "KeepRelative" "KeepRelative" true)
  (return _returnvalue))

(fn `UserConstructionScript`)