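; Dungeon game state that kicks off procedural dungeon generation when play begins.
; It dims or brightens the level's directional light to a fixed intensity, then spawns a SpawnBP generator at a fixed location.
; The generator receives overlapping Wave Function Collapse options and the Less_Rooms input texture.
; It then runs the WFC generation and calls SetSpawn.
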(event `self.ReceiveBeginPlay`
  (`self.Adjust World Settings`)
  (bind _returnvalue (`|SpawnActorFromClass` "/Game/DungeonPuzzleGen/Blueprints/SpawnBP.SpawnBP_C" (`KismetMathLibrary.MakeTransform` (-6000.0 6000.0 200.0)) "Undefined" "OverrideRootScale" null null))
  (bind _output_get (set `self.SpawnBP` _returnvalue))
  (set `SpawnLevel.options` (make `OverlappingWFCOptions` 30 30 true true 8 false 3) _output_get)
  (set `SpawnLevel.InputTexture` "/Game/DungeonPuzzleGen/WFC_Textures/Less_Rooms.Less_Rooms" _output_get)
  (`/Game/DungeonPuzzleGen/Blueprints/SpawnBP.Spawn wfc` _output_get)
  (`/Game/DungeonPuzzleGen/Blueprints/SpawnBP.Set Spawn` _output_get))

(event `Adjust World Settings`
  (bind _returnvalue (`GameplayStatics.GetActorOfClass` "/Script/Engine.DirectionalLight"))
  (`LightComponent.SetIntensity` (`Light.LightComponent` _returnvalue) 2.0))

(fn `UserConstructionScript`)