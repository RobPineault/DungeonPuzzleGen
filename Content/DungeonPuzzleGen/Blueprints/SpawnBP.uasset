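; Dungeon generator actor that runs Wave Function Collapse on BeginPlay and spawns a grid of Tile actors from the resulting Wang indices.
; Tileset supplies each tile's class, rotation and scale, then tiles receive their grid neighbors.
; GetPieces can lift tiles outside the largest piece, but its MakePiece labeling and Search completion check are not wired in.
; An instanced-mesh preview of the WFC color image is also left disconnected.
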(event `self.ReceiveBeginPlay`
  (`KismetSystemLibrary.Delay` 1.0)
  (`self.Spawn wfc`))

(event `Spawn wfc`
  (set `self.seed` (`KismetMathLibrary.RandomInteger` 1000))
  (bind (_colorimg _wangimg) (`self.RunWFC`))
  (set `self.outImage` _colorimg)
  (set `self.outWang` _wangimg)
  (`self.Spawn Wang`))

(event `Spawn outimage`
  (set `self.Index` 0)
  (bind _returnvalue (`KismetSystemLibrary.K2_SetTimerDelegate` (delegate `add instance`) 0.001 true)))

(event `add instance`
  (bind _tilesize (`self.tileSize`))
  (bind _index (`self.Index`))
  (bind _outimage (`self.outImage`))
  (bind (_out_height _out_width) (break `OverlappingWFCOptions` (`self.options`)))
  (bind _output (`|GetArrayItem` _outimage _index))
  (bind _returnvalue (`KismetMathLibrary.Conv_Int64ToDouble` (* (`KismetMathLibrary.Conv_IntToInt64` (mod _index _out_width)) _tilesize)))
  (bind _returnvalue_2 (`KismetMathLibrary.Conv_Int64ToDouble` (* (`KismetMathLibrary.Conv_IntToInt64` (/ _index _out_width)) _tilesize)))
  (bind _returnvalue_3 (`KismetMathLibrary.MakeTransform` (`KismetMathLibrary.MakeVector` _returnvalue _returnvalue_2 -50.0) (struct) (4.0 4.0 1.0)))
  (if (< _index (`KismetArrayLibrary.Array_Length` _outimage))
    (if (== _output (`KismetMathLibrary.LinearColor_Black`))
      (`InstancedStaticMeshComponent.AddInstance` (`self.InstancedStaticMesh`) _returnvalue_3 false)
      (elif (== (`KismetMathLibrary.LinearColor_White`) _output)
        (`InstancedStaticMeshComponent.AddInstance` (`self.InstancedStaticMesh1`) (`KismetMathLibrary.MakeTransform` (`KismetMathLibrary.MakeVector` _returnvalue _returnvalue_2 -225.0) (struct) (4.0 4.0 1.0)) false)
        (else
          (`InstancedStaticMeshComponent.AddInstance` (`self.InstancedStaticMesh2`) _returnvalue_3 false))))
    (`/Engine/EditorBlueprintResources/StandardMacros.IncrementInt` (`self.Index`))
    (else
      (`KismetSystemLibrary.K2_ClearAndInvalidateTimerHandle` (stale `Spawn outimage` _returnvalue)))))

(event `Spawn Wang`
  (bind _tilesize (`self.tileSize`))
  (bind (_out_height _out_width) (break `OverlappingWFCOptions` (`self.options`)))
  (for (_array_element _array_index) (`self.outWang`)
    (bind (_mesh _rotation _scale _newparam) (`/Game/DungeonPuzzleGen/Blueprints/Tileset.Get Wang Mesh` (`self.Tileset`) _array_element))
    (if (`KismetSystemLibrary.IsValidClass` _newparam)
      (bind _returnvalue (`|SpawnActorFromClass` _newparam (`KismetMathLibrary.MakeTransform` (+ (`KismetMathLibrary.MakeVector` (`KismetMathLibrary.Conv_Int64ToDouble` (* (`KismetMathLibrary.Conv_IntToInt64` (mod _array_index _out_width)) _tilesize)) (`KismetMathLibrary.Conv_Int64ToDouble` (* (`KismetMathLibrary.Conv_IntToInt64` (/ _array_index _out_width)) _tilesize))) (`self.K2_GetActorLocation`)) _rotation _scale) "Undefined" "OverrideRootScale" null null))
      (bind _astile (cast `/Game/DungeonPuzzleGen/Blueprints/Tile` _returnvalue))
      (`KismetArrayLibrary.Array_Add` (`self.Tiles`) _astile)))
  (`self.Update Neighbors`))

(event `Update Neighbors`
  (bind _array (`|MakeArray` (struct) :!type "/Game/DungeonPuzzleGen/Blueprints/TileNeighbor Structure"))
  (bind _tiles (`self.Tiles`))
  (bind (_out_height _out_width) (break `OverlappingWFCOptions` (`self.options`)))
  (for (_array_element _array_index) _tiles
    (bind _returnvalue (- _array_index _out_width))
    (if (> _returnvalue 0)
      (`KismetArrayLibrary.Array_Add` _array (make `/Game/DungeonPuzzleGen/Blueprints/TileNeighbor` (`|GetArrayItem` _tiles _returnvalue))))
    (if (!= (mod _array_index _out_width) (- _out_width 1))
      (`KismetArrayLibrary.Array_Add` _array (make `/Game/DungeonPuzzleGen/Blueprints/TileNeighbor` (`|GetArrayItem` _tiles (+ _array_index 1)) "NewEnumerator1")))
    (if (!= (/ _array_index _out_width) _out_height)
      (`KismetArrayLibrary.Array_Add` _array (make `/Game/DungeonPuzzleGen/Blueprints/TileNeighbor` (`|GetArrayItem` _tiles (+ _array_index _out_width)) "NewEnumerator2")))
    (if (!= (mod _array_index _out_width) 0)
      (`KismetArrayLibrary.Array_Add` _array (make `/Game/DungeonPuzzleGen/Blueprints/TileNeighbor` (`|GetArrayItem` _tiles (- _array_index 1)) "NewEnumerator3"))
      (`/Game/DungeonPuzzleGen/Blueprints/Tile.Set Neighbors` _array_element _array self)))
  (`self.Neighbors Set`)
  (`self.Get Pieces`))

(event `Get Pieces`
  (for _array_element (`self.Tiles`)
    (set `/Game/DungeonPuzzleGen/Blueprints/Tile.Visited` false _array_element))
  (set `self.Piece Count` 0)
  (while (not (`self.Complete`))
    _)
  (`KismetSystemLibrary.Delay` 1.0)
  (`KismetSystemLibrary.PrintString` (`KismetStringLibrary.Conv_IntToString` (`self.Piece Count`)))
  (`KismetSystemLibrary.PrintString` (`KismetStringLibrary.Conv_IntToString` (`self.Max Piece Value`)))
  (if (`self.Large Piece Only`)
    (for _array_element_2 (`self.Tiles`)
      (if (!= (`/Game/DungeonPuzzleGen/Blueprints/Tile.Piece Number` _array_element_2) (`self.Max Piece Value`))
        (`self.K2_TeleportTo` :`self` _array_element_2 :`DestLocation` (+ (`self.K2_GetActorLocation` _array_element_2) (0.0 0.0 400.0)))))))

(event `Make piece`
  (bind _piece_count (`self.Piece Count`))
  (for _array_element (`self.Tiles`)
    (if (or (not (`/Game/DungeonPuzzleGen/Blueprints/Tile.Visited` _array_element)) (!= (`/Game/DungeonPuzzleGen/Blueprints/Tile.Tile Type` _array_element) 0))
      (bind _count_out (`/Game/DungeonPuzzleGen/Blueprints/Tile.Visit` _piece_count))
      (if (< (`self.Max Piece Size`) _count_out)
        (set `self.Max Piece Size` _count_out)
        (set `self.Max Piece Value` _piece_count)
        (break)
        (else
          (`/Engine/EditorBlueprintResources/StandardMacros.IncrementInt` _piece_count))))))

(fn `Add Or Create`
  (params (mesh :type "StaticMesh Object Reference"))
  (returns (NewParam :type "InstancedStaticMeshComponent Object Reference"))
  (for _array_element (`self.K2_GetComponentsByClass` "/Script/Engine.InstancedStaticMeshComponent")
    (if (== mesh (`StaticMeshComponent.StaticMesh` _array_element))
      (return _array_element)))
  (bind _returnvalue (`AddComponent|NODE_AddInstancedStaticMeshComponent-0`))
  (`StaticMeshComponent.SetStaticMesh` _returnvalue mesh)
  (return _returnvalue))

(fn `Get Neighbors`
  (params (`Color 1` :type Integer))
  (returns (NewParam :type "Map of /Game/DungeonPuzzleGen/Blueprints/Direction Enum to Object Object Reference"))
  (return))

(fn `Search`
  (returns (Complete :type Boolean))
  (for _array_element (`self.Tiles`)
    (if (and (not (`/Game/DungeonPuzzleGen/Blueprints/Tile.Visited` _array_element)) (!= (`/Game/DungeonPuzzleGen/Blueprints/Tile.Tile Type` _array_element) 0))
      (return false)))
  (return true))

(fn `UserConstructionScript`)