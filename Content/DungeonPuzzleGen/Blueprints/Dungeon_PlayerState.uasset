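; Player state for a dungeon puzzle game that tracks health and gold and drives the HUD, death and respawn.
; Damage updates the health widget and starts a short timer-based immunity, or at zero destroys the character, resets gold and torch, and asks the GameState's SpawnBP to respawn.
; SpawnPlayer spawns and possesses a fresh first-person character.
; The first gold pickup activates the exit, and reaching it shows an objective widget and the mouse cursor.
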(event `self.ReceiveBeginPlay`
  (`self.Init Healthbar`))

(event `Init Healthbar`
  (bind _returnvalue (`|CreateWidget` "/Game/DungeonPuzzleGen/Blueprints/Health.Health_C"))
  (`UserWidget.AddToViewport` _returnvalue 0)
  (bind _output_get (set `self.Health Widget` _returnvalue))
  (set `/Game/DungeonPuzzleGen/Blueprints/Health.Health Percent` 1.0 _output_get))

(event `Take Damage`
  (params (amount :type Integer))
  (if (not (`self.Immune`))
    (bind _output_get (set `self.Health` (`KismetMathLibrary.Clamp` (- (`self.Health`) amount) 0 (`KismetMathLibrary.FTrunc` (`self.Max Health`)))))
    (set `/Game/DungeonPuzzleGen/Blueprints/Health.Health Percent` (/ _output_get (`self.Max Health`)) (`self.Health Widget`))
    (if (== _output_get 0)
      (`self.Die`)
      (else
        (set `self.Immune` true)
        (`KismetSystemLibrary.K2_SetTimerDelegate` (delegate `End Immunity`) 2.0)))))

(event `End Immunity`
  (set `self.Immune` false))

(event `Spawn Player`
  (params (Transform :type "Transform Structure"))
  (set `self.Health` (`KismetMathLibrary.FTrunc` (`self.Max Health`)))
  (`self.Init Healthbar`)
  (bind _returnvalue (`|SpawnActorFromClass` "/Game/FirstPerson/Blueprints/BP_FirstPersonCharacter.BP_FirstPersonCharacter_C" Transform "Undefined" "OverrideRootScale" null null))
  (`Controller.Possess` (`GameplayStatics.GetPlayerController` 0) _returnvalue))

(event `Die`
  (`Pawn.DetachFromControllerPendingDestroy` (`GameplayStatics.GetPlayerPawn` 0))
  (bind _returnvalue (`GameplayStatics.GetActorOfClass` "/Game/FirstPerson/Blueprints/BP_FirstPersonCharacter.BP_FirstPersonCharacter_C"))
  (`self.K2_DestroyActor` _returnvalue)
  (bind _asdungeon_game_state (cast `/Game/DungeonPuzzleGen/Blueprints/DungeonGameState` (`GameplayStatics.GetGameState`)))
  (bind _output_get (set `self.Gold` 0))
  (`/Game/DungeonPuzzleGen/Blueprints/Health.Update GOld` (`self.Health Widget`) _output_get)
  (set `self.Holding Torch` false)
  (`/Game/DungeonPuzzleGen/Blueprints/SpawnBP.Respawn` (`/Game/DungeonPuzzleGen/Blueprints/DungeonGameState.SpawnBP` _asdungeon_game_state)))

(event `Reach Exit`
  (bind _returnvalue (`|CreateWidget` "/Game/DungeonPuzzleGen/Blueprints/ObjectiveWidget.ObjectiveWidget_C"))
  (`UserWidget.AddToViewport` _returnvalue 0)
  (bind _asmouse_controller (cast `/Game/DungeonPuzzleGen/Blueprints/MouseController` (`GameplayStatics.GetPlayerController` 0)))
  (`/Game/DungeonPuzzleGen/Blueprints/MouseController.Show Mouse` _asmouse_controller))

(event `Pick Up Gold`
  (bind _gold (`self.Gold`))
  (if (== _gold 0)
    (bind _asdungeon_game_state (cast `/Game/DungeonPuzzleGen/Blueprints/DungeonGameState` (`GameplayStatics.GetGameState`)))
    (`/Game/DungeonPuzzleGen/Blueprints/RuinsTiles/Tile1.Set As Exit` (`/Game/DungeonPuzzleGen/Blueprints/SpawnBP.Exit` (`/Game/DungeonPuzzleGen/Blueprints/DungeonGameState.SpawnBP` _asdungeon_game_state))))
  (bind _result (`/Engine/EditorBlueprintResources/StandardMacros.IncrementInt` _gold)
    (:`  `
      (`/Game/DungeonPuzzleGen/Blueprints/Health.Update GOld` (`self.Health Widget`) _result))))

(fn `Update Health`
  (params (`New Health` :type "Float (double-precision)") (Widget :type "/Game/DungeonPuzzleGen/Blueprints/Health Object Reference"))
  (returns (Health :type "Float (double-precision)"))
  (bind _output_get (set `self.Health` (`KismetMathLibrary.FTrunc` (`KismetMathLibrary.FClamp` `New Health` 0.0 (`self.Max Health`)))))
  (if (`KismetSystemLibrary.IsValid` Widget)
    (set `/Game/DungeonPuzzleGen/Blueprints/Health.Health Percent` (/ _output_get (`self.Max Health`)) Widget))
  (return (`KismetMathLibrary.Conv_IntToDouble` _output_get)))

(fn `UserConstructionScript`)