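; Tileset Blueprint that maps a Wang tile value to a static mesh, rotation, scale and tile actor for dungeon puzzle generation.
; GetWangMesh searches each tile's Options for the value and, for two- or four-option tiles, derives yaw from the option index in quarter turns.
; Unmatched values are printed and fall back to Option_Void.
; ContainsInt is a helper that tests whether an option list holds a value.
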(event `self.ReceiveBeginPlay`)

(fn `contains int`
  (params (NewParam :type Integer) (NewParam1 :type "Array of /Game/DungeonPuzzleGen/Blueprints/WangTile Structure"))
  (returns (NewParam2 :type Boolean))
  (for _array_element NewParam1
    (bind _returnvalue (== NewParam (`.Value_2_DB6B906F46D925C55A2FAD97043C2901` (break `/Game/DungeonPuzzleGen/Blueprints/WangTile` _array_element))))
    (if _returnvalue
      (return _returnvalue)))
  (return false))

(fn `Get Wang Mesh`
  (params (wang :type Integer))
  (returns (mesh :type "StaticMesh Object Reference") (rotation :type "Rotator Structure") (scale :type "Vector Structure") (NewParam :type "Actor Class Reference"))
  (for _array_element (`.Tileset_3_4811465E4709AADE59B969A710AE5D41` (break `/Game/DungeonPuzzleGen/Blueprints/TilesetStruct` (`self.Tiles`)))
    (bind (_name _options _staticmesh _tileactor) (break `/Game/DungeonPuzzleGen/Blueprints/WangData` _array_element))
    (for (_array_element_2 _array_index) _options
      (bind (_value _rotation _scale) (break `/Game/DungeonPuzzleGen/Blueprints/WangTile` _array_element_2))
      (if (== wang _value)
        (switch `int` (`KismetArrayLibrary.Array_Length` _options)
          (:`1`
            (return _staticmesh (struct) _scale _tileactor))
          (:`2`
            _)
          (:`4`
            _))
        (return _staticmesh (`KismetMathLibrary.MakeRotator` 0.0 0.0 (`KismetMathLibrary.Conv_IntToDouble` (* _array_index 90))) _scale _tileactor))))
  (`KismetSystemLibrary.PrintString` (`KismetStringLibrary.Conv_IntToString` wang))
  (return "/WaveFunctionCollapse/Core/SpecialOptions/Option_Void.Option_Void" (struct) (1.0 1.0 1.0) null))