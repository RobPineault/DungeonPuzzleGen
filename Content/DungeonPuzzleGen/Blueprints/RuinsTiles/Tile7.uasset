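; Ruins tile Blueprint for dungeon generation that randomly dresses itself as either walls or a corner piece on BeginPlay.
; Usually it builds left and bottom rock walls three high, then attaches a random Walls composition to the last child component of each.
; Otherwise it spawns a corner composition on the floor and attaches a tall rock wall mesh at every socket of that component.
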(event `self.ReceiveBeginPlay`
  (bind _wall_left_base (`self.Wall Left Base`))
  (bind _wall_bottom_base (`self.Wall Bottom Base`))
  (bind _children (`SceneComponent.GetChildrenComponents` _wall_bottom_base true))
  (bind _children_2 (`SceneComponent.GetChildrenComponents` _wall_left_base true))
  (if (`KismetMathLibrary.RandomBoolWithWeight` 0.75)
    (set `self.Wall Height` 3)
    (`self.Build Wall` _wall_left_base "/Game/DungeonPuzzleGen/Meshes/LostRuinTileset/SM_Rock_Wall__Base_6X1.SM_Rock_Wall__Base_6X1")
    (bind _asstatic_mesh_component (cast `StaticMeshComponent` (`|GetArrayItem` _children_2 (`KismetArrayLibrary.Array_LastIndex` _children_2))))
    (`self.Create SMC From Comp` (`KismetArrayLibrary.Array_Random` (`self.Walls`)) _asstatic_mesh_component)
    (`self.Build Wall` _wall_bottom_base "/Game/DungeonPuzzleGen/Meshes/LostRuinTileset/SM_Rock_Wall__Base_6X1.SM_Rock_Wall__Base_6X1")
    (bind _asstatic_mesh_component_2 (cast `StaticMeshComponent` (`|GetArrayItem` _children (`KismetArrayLibrary.Array_LastIndex` _children))))
    (`self.Create SMC From Comp` (`KismetArrayLibrary.Array_Random` (`self.Walls`)) _asstatic_mesh_component_2)
    (else
      (bind _child (`self.Create SMC From Comp` (`self.Corner Composition`) (`self.Floor Base`)))
      (for _array_element (`SceneComponent.GetAllSocketNames` _child)
        (`self.Create SMC From Mesh` "/Game/ModularLostRuinKit/Models/Structure/WFoliage/SM_Rock_Wall_1X1_Tall_Fol.SM_Rock_Wall_1X1_Tall_Fol" _child _array_element)))))

(fn `UserConstructionScript`)