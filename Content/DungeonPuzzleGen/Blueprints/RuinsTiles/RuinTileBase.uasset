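; Base ruins tile for the procedural dungeon, providing shared wall, treasure, spike and dead-end dressing logic.
; BuildWall stacks rock meshes to WallHeight on alternating sockets, rolling torch placement from tile rates and the GameState spawner's global rate.
; Events scatter randomly placed treasure, put a broken barrel on dead ends, or attach a single Spikes actor that replaces the visible floor, rotated for one tile type.
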(event `Spawn Treasure`
  (for _ (range (+ (`KismetMathLibrary.RandomInteger` 4) 1))
    (`|SpawnActorFromClass` "/Game/DungeonPuzzleGen/Blueprints/Treasure.Treasure_C" (`KismetMathLibrary.MakeTransform` (+ (.location (`self.GetTransform`)) (`KismetMathLibrary.MakeVector` (`KismetMathLibrary.RandomFloatInRange` -290.0 290.0) (`KismetMathLibrary.RandomFloatInRange` -290.0 290.0) 25.0)) (`KismetMathLibrary.MakeRotator` 0.0 0.0 (`KismetMathLibrary.RandomFloatInRange` 0.0 359.0))) "Undefined" "OverrideRootScale" null null)))

(event `Mark as path`
  (params (`Dead end` :type Boolean))
  (if `Dead end`
    (`self.Create SMC From Mesh` "/Game/ModularLostRuinKit/Models/Props/WithFoliage/SM_Barrel_Broken4_Fol.SM_Barrel_Broken4_Fol" (`self.Floor Base`) "Center")))

(event `Add Spikes`
  (params (offset :type "Float (double-precision)") (moving :type Boolean) (Type :type "/Game/DungeonPuzzleGen/Blueprints/Traps/PlatformType Enum" :default "NewEnumerator0") (flip :type Boolean))
  (if (not (`self.With Spikes`))
    (bind _returnvalue (`|SpawnActorFromClass` "/Game/DungeonPuzzleGen/Blueprints/Traps/Spikes.Spikes_C" (select `bool` (== (`self.Tile Type`) 68) :`false` (`KismetMathLibrary.MakeTransform` (0.0 0.0 0.0)) :`true` (`KismetMathLibrary.MakeTransform` (0.0 0.0 0.0) (struct :`Yaw` 180.0))) "Undefined" "OverrideRootScale" null offset moving Type flip null))
    (`self.K2_AttachToComponent` _returnvalue (`self.Floor Base`) "Center" "KeepRelative" "KeepRelative" "KeepRelative" true)
    (`SceneComponent.SetVisibility` (`self.Floor Base`) false false)
    (set `self.With Spikes` true)))

(fn `Build Wall`
  (params (`Wall base` :type "StaticMeshComponent Object Reference") (`Wall SM` :type "StaticMesh Object Reference") (NewParam :type "StaticMesh Object Reference"))
  (locals (`Last Wall Comp` :type "StaticMeshComponent Object Reference") (`Torch Spawned` :type Boolean) (`With Torch` :type Boolean) (`Torch Index` :type Integer))
  (`StaticMeshComponent.SetStaticMesh` `Wall base` `Wall SM`)
  (set `local.Last Wall Comp` `Wall base`)
  (bind _asdungeon_game_state (cast `/Game/DungeonPuzzleGen/Blueprints/DungeonGameState` (`GameplayStatics.GetGameState`)))
  (bind _output_get (set `local.With Torch` (`KismetMathLibrary.RandomBoolWithWeight` (* (`self.Torch Spawn Rate`) (`/Game/DungeonPuzzleGen/Blueprints/SpawnBP.Global Torch Rate` (`/Game/DungeonPuzzleGen/Blueprints/DungeonGameState.SpawnBP` _asdungeon_game_state))))))
  (if _output_get
    (if (`KismetMathLibrary.RandomBoolWithWeight` (`self.Torch Middle Rate`))
      (set `local.Torch Index` 1)
      (else
        (bind _output_get_2 (set `local.Torch Index` (* (`KismetMathLibrary.RandomInteger` 1) 2)))
        (if (== _output_get_2 0)
          (`self.Spawn Actor from SMC` "/Game/ModularLostRuinKit/Blueprint/Props/BP_Torch.BP_Torch_C" "Torch Center R" (`local.Last Wall Comp`))))))
  (for _index (range 1 (+ (`self.Wall Height`) 1))
    (bind _child (`self.Create SMC From Mesh` "/Game/DungeonPuzzleGen/Meshes/LostRuinTileset/SM_Rock_Wall__Base_6X1.SM_Rock_Wall__Base_6X1" (`local.Last Wall Comp`) (select `int` (mod _index 2) :`0` "Wall T" :`1` "Wall T R")))
    (if (and (== _index (`local.Torch Index`)) (`local.With Torch`))
      (`self.Spawn Actor from SMC` "/Game/ModularLostRuinKit/Blueprint/Props/BP_Torch.BP_Torch_C" "Torch Center" _child))
    (set `local.Last Wall Comp` _child)))

(fn `UserConstructionScript`
  (`parent.UserConstructionScript`))