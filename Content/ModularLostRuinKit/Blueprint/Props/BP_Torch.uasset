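; BP_Torch is a torch prop that the first-person character can pick up and hold.
; Overlapping its capsule stores the character and binds to that character's OnItemTake dispatcher.
; OnTake snaps the torch to the GripPoint socket on the first-person mesh, sets a fixed scale and rotation, and disables the static mesh's collision.
; The binding is never removed when the overlap ends.
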(event `self.Capsule.OnComponentBeginOverlap`
  (params (OverlappedComponent :type "PrimitiveComponent Object Reference") (OtherActor :type "Actor Object Reference") (OtherComp :type "PrimitiveComponent Object Reference") (OtherBodyIndex :type Integer) (bFromSweep :type Boolean) (SweepResult :type "HitResult Structure (by ref)"))
  (bind _asbp_first_person_character (cast `/Game/FirstPerson/Blueprints/BP_FirstPersonCharacter` OtherActor))
  (bind _output_get (set `self.Person Character` _asbp_first_person_character))
  (add `/Game/FirstPerson/Blueprints/BP_FirstPersonCharacter.OnItemTake` _output_get (`|CreateDelegate` :!event `On Take`)))

(event `On Take`
  (`self.K2_AttachToComponent` self (`/Game/FirstPerson/Blueprints/BP_FirstPersonCharacter.FirstPersonMesh` (`self.Person Character`)) "GripPoint" "SnapToTarget" "SnapToTarget" "SnapToTarget" true)
  (`self.SetActorScale3D` (0.75 0.75 0.75))
  (`self.K2_SetActorRotation` (struct :`Pitch` 100.0))
  (`PrimitiveComponent.SetCollisionEnabled` (`self.StaticMesh`) "NoCollision"))

(fn `UserConstructionScript`)